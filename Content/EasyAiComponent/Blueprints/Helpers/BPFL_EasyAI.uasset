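; Blueprint function library of EasyAI helpers for broadcasting noises to AI and applying damage.
; MakeNoiseAtLocation draws debug spheres, then sends a noise event to each pawn's BP_EasyAiComponent, using a sphere overlap within MaxRange or every pawn when the range is zero or less.
; DamageActor calls Hurt on the target's BPC_Damageable component and returns whether that component was found.
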(fn `DamageActor`
  (params (DamagedActor :type "Actor Object Reference") (Damage :type "Float (double-precision)") (DamagingActor :type "Actor Object Reference"))
  (returns (`ActorDamaged?` :type Boolean))
  (bind _returnvalue (`Actor.GetComponentByClass` DamagedActor "/Game/EasyAiComponent/Blueprints/OtherComponents/Damageable/BPC_Damageable.BPC_Damageable_C"))
  (`/Engine/EditorBlueprintResources/StandardMacros.IsValid` _returnvalue
    (:`Is Valid`
      (`/Game/EasyAiComponent/Blueprints/OtherComponents/Damageable/BPC_Damageable.Hurt` _returnvalue Damage DamagingActor)
      (return true))
    (:`Is Not Valid`
      (return false))))

(fn `MakeNoiseAtLocation`
  (params (NoiseLocation :type "Vector Structure") (Instigator :type "Actor Object Reference") (MaxRange :type "Float (double-precision)" :default 0.0) (OverrideNoiseAsEnemy :type Boolean))
  (`KismetSystemLibrary.DrawDebugSphere` null NoiseLocation 50.0 12 (struct :`G` 1.0 :`B` 0.173102 :`A` 1.0) 1.0)
  (`KismetSystemLibrary.DrawDebugSphere` null NoiseLocation MaxRange 12 (struct :`R` 0.630208 :`G` 1.0 :`B` 0.69422 :`A` 1.0) 1.0)
  (if (<= MaxRange 0.0)
    (bind _outactors (`GameplayStatics.GetAllActorsOfClass` null "/Script/Engine.Pawn"))
    (for _array_element _outactors
      (bind _returnvalue (`Actor.GetComponentByClass` _array_element "/Game/EasyAiComponent/BP_EasyAiComponent.BP_EasyAiComponent_C"))
      (`/Engine/EditorBlueprintResources/StandardMacros.IsValid` _returnvalue
        (:`Is Valid`
          (`/Game/EasyAiComponent/BP_EasyAiComponent.OnRecieveNoiseEvent` _returnvalue NoiseLocation Instigator OverrideNoiseAsEnemy))))
    (else
      (bind _outactors_2 (`KismetSystemLibrary.SphereOverlapActors` null NoiseLocation MaxRange (`|MakeArray` "ObjectTypeQuery3" :!type "EObjectTypeQuery Enum") "/Script/Engine.Pawn"))
      (for _array_element_2 _outactors_2
        (bind _returnvalue_2 (`Actor.GetComponentByClass` _array_element_2 "/Game/EasyAiComponent/BP_EasyAiComponent.BP_EasyAiComponent_C"))
        (`/Engine/EditorBlueprintResources/StandardMacros.IsValid` _returnvalue_2
          (:`Is Valid`
            (`/Game/EasyAiComponent/BP_EasyAiComponent.OnRecieveNoiseEvent` _returnvalue_2 NoiseLocation Instigator OverrideNoiseAsEnemy)))))))