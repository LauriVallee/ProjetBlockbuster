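; Gradual detection component that gives Easy AI enemies a fill-up delay before they fully detect the owning actor.
; It creates a detection bar widget, and StartDetection and StopDetection set its target to full or empty.
; A gated Tick moves the bar at a constant rate.
; A full bar turns red and confirms detection; an empty one hides after a delay and sends the AI to investigate the owner's location.
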(event `self.ReceiveBeginPlay`
  ; Create Detection widget, can replace with custom widget
  (bind _returnvalue (`|CreateWidget` "/Game/EasyAiComponent/Blueprints/OtherComponents/GradualDetection/Widgets/WBP_Detection.WBP_Detection_C"))
  (bind _output_get (set `self.DetectionWidget` _returnvalue))
  (`UserWidget.AddToViewport` _output_get 0))

(event `/Game/EasyAiComponent/Blueprints/Helpers/BPI_EasyAI.StartDetection`
  (params (AI :type "Pawn Object Reference"))
  (bind _detectionbar (`/Game/EasyAiComponent/Blueprints/OtherComponents/GradualDetection/Widgets/WBP_Detection.DetectionBar` (`self.DetectionWidget`)))
  ; Event when enemy AI sees player, starts filling detection
  (set `/Game/EasyAiComponent/Blueprints/OtherComponents/GradualDetection/Widgets/WBP_Detection.AI` AI (`self.DetectionWidget`))
  (switch `ESlateVisibility` (`Widget.GetVisibility` _detectionbar)
    (:`Visible`
      _)
    (:`Hidden`
      (`Widget.SetVisibility` _detectionbar "Visible")))
  (set `self.TargetPercent` 1.0)
  (`self.OpenGate`))

(event `/Game/EasyAiComponent/Blueprints/Helpers/BPI_EasyAI.StopDetection`
  ; Event when enemy loses sight of player, starts decreasing detection
  (set `self.TargetPercent` 0.0)
  (`self.OpenGate`))

(event `self.ReceiveTick`
  (params (DeltaSeconds :type "Float (single-precision)"))
  ; Gradual Detection Behavior
  (`/Engine/EditorBlueprintResources/StandardMacros.Gate` true :!label _label
    (:`Exit`
      ;; Interpolates the slider value of widget at st detection rate
      (`ProgressBar.SetPercent` (`/Game/EasyAiComponent/Blueprints/OtherComponents/GradualDetection/Widgets/WBP_Detection.DetectionBar` (`self.DetectionWidget`)) (`KismetMathLibrary.FInterpTo_Constant` (`ProgressBar.Percent` (`/Game/EasyAiComponent/Blueprints/OtherComponents/GradualDetection/Widgets/WBP_Detection.DetectionBar` (`self.DetectionWidget`))) (`self.TargetPercent`) DeltaSeconds (`self.DetectionRate`)))
      ;; If progress is completely filled or completely empty
      (if (== (`ProgressBar.Percent` (`/Game/EasyAiComponent/Blueprints/OtherComponents/GradualDetection/Widgets/WBP_Detection.DetectionBar` (`self.DetectionWidget`))) (`self.TargetPercent`))
        (`self.CloseGate`)
        (if (select `int` (`KismetMathLibrary.Round` (`self.TargetPercent`)) :`0` true :`1` false)
          ;; Behavior if detection is emptied
          (`KismetSystemLibrary.RetriggerableDelay` 0.5)
          (`Widget.SetVisibility` (`/Game/EasyAiComponent/Blueprints/OtherComponents/GradualDetection/Widgets/WBP_Detection.DetectionBar` (`self.DetectionWidget`)) "Hidden")
          (`ProgressBar.SetFillColorAndOpacity` (`/Game/EasyAiComponent/Blueprints/OtherComponents/GradualDetection/Widgets/WBP_Detection.DetectionBar` (`self.DetectionWidget`)) (struct :`R` 1.0 :`G` 1.0 :`B` 1.0 :`A` 1.0))
          (`/Game/EasyAiComponent/BP_EasyAiComponent.SetStateAsInvestigative` (`Actor.GetComponentByClass` (`/Game/EasyAiComponent/Blueprints/OtherComponents/GradualDetection/Widgets/WBP_Detection.AI` (`self.DetectionWidget`)) "/Game/EasyAiComponent/BP_EasyAiComponent.BP_EasyAiComponent_C") (`Actor.K2_GetActorLocation` (`self.GetOwner`)))
          (set `/Game/EasyAiComponent/Blueprints/OtherComponents/GradualDetection/Widgets/WBP_Detection.AI` null (`self.DetectionWidget`))
          (else
            ;; Behavior if detection is filled
            (`ProgressBar.SetFillColorAndOpacity` (`/Game/EasyAiComponent/Blueprints/OtherComponents/GradualDetection/Widgets/WBP_Detection.DetectionBar` (`self.DetectionWidget`)) (struct :`R` 1.0 :`B` 0.021698 :`A` 1.0))
            (`/Game/EasyAiComponent/BP_EasyAiComponent.OnEnemyGradualDetected` (`Actor.GetComponentByClass` (`/Game/EasyAiComponent/Blueprints/OtherComponents/GradualDetection/Widgets/WBP_Detection.AI` (`self.DetectionWidget`)) "/Game/EasyAiComponent/BP_EasyAiComponent.BP_EasyAiComponent_C"))))))))

(event `OpenGate`
  ; Gradual Detection Behavior
  (goto _label :!via `Open`))

(event `CloseGate`
  ; Gradual Detection Behavior
  (goto _label :!via `Close`))

(fn `GetPatrolRoute`
  (returns (PatrolRoute :type "/Game/EasyAiComponent/Blueprints/BP_PatrolRoute Object Reference"))
  (return null))

(fn `SetMovementSpeed`
  (params (Speed :type "/Game/EasyAiComponent/Enums/E_MovementSpeed Enum" :default "NewEnumerator0"))
  (returns (SpeedValue :type "Float (double-precision)"))
  (return 0.0))