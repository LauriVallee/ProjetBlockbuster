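; Actor component that gives its owner health and handles damage and healing, part of the EasyAiComponent set.
; Health starts at MaxHealth on BeginPlay.
; Hurt and Heal clamp the value between zero and MaxHealth, then broadcast dispatchers: OnDeath when health reaches zero, otherwise OnHurt with damage and instigating actor, or OnHeal after healing.
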(event `self.ReceiveBeginPlay`
  (set `self.Health` (`self.MaxHealth`)))

(fn `Heal`
  (params (Heal :type "Float (double-precision)"))
  (set `self.Health` (`KismetMathLibrary.FClamp` (+ (`self.Health`) Heal) 0.0 (`self.MaxHealth`)))
  (`self.OnHeal`))

(fn `Hurt`
  (params (Damage :type "Float (double-precision)") (DamagingActor :type "Actor Object Reference"))
  (bind _output_get (set `self.Health` (`KismetMathLibrary.FClamp` (- (`self.Health`) Damage) 0.0 (`self.MaxHealth`))))
  (if (<= _output_get 0.0)
    (`self.OnDeath`)
    (else
      (`self.OnHurt` Damage DamagingActor))))