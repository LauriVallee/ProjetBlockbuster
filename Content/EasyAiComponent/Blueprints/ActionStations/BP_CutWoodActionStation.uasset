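; Wood-cutting action station from the Easy AI component, where a character performs repeated chopping until the station is used up.
; BeginPlay picks a small random use limit.
; UseActionStation plays the melee attack montage on the user's owning Character, waits on a fixed delay, increments the use count and calls itself again.
; At the limit it notifies the user component that the action is finished and destroys itself.
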(event `self.ReceiveBeginPlay`
  (`parent.ReceiveBeginPlay`)
  (set `self.MaxUseNbr` (`KismetMathLibrary.RandomInteger` 3)))

(event `self.UseActionStation`
  (params (User :type "/Game/EasyAiComponent/BP_EasyAiComponent Object Reference"))
  (bind _ascharacter (cast `Character` (`ActorComponent.GetOwner` User)))
  (`Character.PlayAnimMontage` _ascharacter "/Game/EasyAiComponent/Demo/Characters/Great_Sword/AM_MeleeAttack.AM_MeleeAttack" 1.0 "None")
  (`KismetSystemLibrary.Delay` 2.0)
  (bind _result (`/Engine/EditorBlueprintResources/StandardMacros.IncrementInt` (`self.CurrentUseNbr`))
    (:`  `
      (if (>= _result (`self.MaxUseNbr`))
        (`/Game/EasyAiComponent/BP_EasyAiComponent.HandleActionStationFinished` User)
        (`self.K2_DestroyActor`)
        (else
          (`self.UseActionStation` User))))))

(fn `UserConstructionScript`
  (`parent.UserConstructionScript`))