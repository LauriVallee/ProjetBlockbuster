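; BP_PlayMontageCombatAction is an Easy AI combat action that plays an animation montage on the AI's owning character.
; When the action starts, it casts the component's owner to Character and plays the configured montage on its mesh at the configured play rate.
; The action ends whether the montage completes or is interrupted; if the owner is not a Character, it stops without ending the action.
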(event `self.StartCombatAction`
  (params (EasyAIComponent :type "/Game/EasyAiComponent/BP_EasyAiComponent Object Reference"))
  (bind _ascharacter (cast `Character` (`ActorComponent.GetOwner` EasyAIComponent)))
  (`|PlayMontage` (`Character.Mesh` _ascharacter) (`self.Montage to Play`) (`self.PlayRate`)
    (:`OnCompleted`
      _)
    (:`OnInterrupted`
      _))
  (`self.EndCombatAction`))

(fn `UserConstructionScript`
  (`parent.UserConstructionScript`))