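; BP_TeleportBackwards is an Easy AI combat action that blinks the AI component's owner a short distance backwards along its forward vector.
; On StartCombatAction it spawns a BP_Burst at the start position, teleports the owner without a sweep, then spawns a second burst at the destination.
; A brief delay follows before it calls EndCombatAction.
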(event `self.StartCombatAction`
  (params (EasyAIComponent :type "/Game/EasyAiComponent/BP_EasyAiComponent Object Reference"))
  (bind _returnvalue (`ActorComponent.GetOwner` EasyAIComponent))
  (`|SpawnActorFromClass` "/Game/EasyAiComponent/Demo/Characters/Great_Sword/BP_Burst.BP_Burst_C" (`self.GetTransform` _returnvalue) "AlwaysSpawn" "MultiplyWithRoot" null null)
  (`self.K2_SetActorLocation` _returnvalue (- (`self.K2_GetActorLocation` _returnvalue) (* (`self.GetActorForwardVector` _returnvalue) 200.0)) false true)
  (`|SpawnActorFromClass` "/Game/EasyAiComponent/Demo/Characters/Great_Sword/BP_Burst.BP_Burst_C" (`self.GetTransform` _returnvalue) "AlwaysSpawn" "MultiplyWithRoot" null null)
  (`KismetSystemLibrary.Delay` 0.5)
  (`self.EndCombatAction`))

(fn `UserConstructionScript`
  (`parent.UserConstructionScript`))