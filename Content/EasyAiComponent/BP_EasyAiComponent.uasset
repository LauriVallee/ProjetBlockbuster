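; Actor component that turns a pawn into an EasyAI agent, running a main behavior tree with per-behavior subtrees injected by gameplay tag.
; A per-tick EQS sight query with optional gradual detection, range-checked noise events and damage events drive a blackboard state: passive, investigating, attacking or dead.
; Faction data filters sight and hearing targets.
; It also optionally adds a damageable component, spawns combat actions, sets movement speed and draws debug views.
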(event `self.ReceiveBeginPlay`
  ; Initialization
  (`self.InitializeVariables`)
  (`self.InitializeBlackboardValues`)
  (`self.InitializeBehaviors`)
  ;[0.15 0.02657 0.01161 0.5] adds Damageable component if can be damaged is true
  (if (`self.IsDamageable`)
    (bind _returnvalue (`|AddComponentByClass` (`self.OwnerActor`) "/Game/EasyAiComponent/Blueprints/OtherComponents/Damageable/BPC_Damageable.BPC_Damageable_C" (`self.MaxHealth`)))
    (add `/Game/EasyAiComponent/Blueprints/OtherComponents/Damageable/BPC_Damageable.OnHurt` _returnvalue (delegate `OnDamaged`))
    (add `/Game/EasyAiComponent/Blueprints/OtherComponents/Damageable/BPC_Damageable.OnDeath` _returnvalue (delegate `OnDeath_Event`))
    (add `/Game/EasyAiComponent/Blueprints/OtherComponents/Damageable/BPC_Damageable.OnHeal` _returnvalue (delegate `OnHeal_Event`))))

(event `OnHeal_Event`
  ;[0.15 0.02657 0.01161 0.5] adds Damageable component if can be damaged is true
  ;; Event on heal
  (`self.OnHeal`))

(event `OnDamaged`
  (params (Damage :type "Float (double-precision)") (DamagingActor :type "Actor Object Reference"))
  ;[0.15 0.02657 0.01161 0.5] adds Damageable component if can be damaged is true
  ;; Event on Damaged
  (`self.HandleSensedDamage` DamagingActor)
  (`self.OnHurt` Damage))

(event `OnDeath_Event`
  ;[0.15 0.02657 0.01161 0.5] adds Damageable component if can be damaged is true
  ;; Event on death
  (`self.OnDeath`)
  (`self.SetStateAsDead`))

(event `self.ReceiveTick`
  (params (DeltaSeconds :type "Float (single-precision)"))
  (bind _sightconeangle (`self.SightConeAngle`))
  (bind _owneractor (`self.OwnerActor`))
  (bind (_returnvalue_x _returnvalue_y _returnvalue_z) (`KismetMathLibrary.BreakVector` (`Actor.K2_GetActorLocation` _owneractor)))
  ;[0 0.6252 0.849 0.5] Sight System
  ;; Handle Sight using EQS query that compare forward vector with DOT Product
  (bind _returnvalue (`EnvQueryManager.RunEQSQuery` "/Game/EasyAiComponent/BehaviorTrees/EQS/EQS_Sight.EQS_Sight" (`self.OwnerAIController`) "SingleResult"))
  (`EnvQueryInstanceBlueprintWrapper.SetNamedParam` _returnvalue "SightRange" (`self.SightRange`))
  (`EnvQueryInstanceBlueprintWrapper.SetNamedParam` _returnvalue "SightConeAngle" (`KismetMathLibrary.MapRangeClamped` (`self.SightConeAngle`) 45.0 1.0 0.7 0.999))
  (add `EnvQueryInstanceBlueprintWrapper.OnQueryFinishedEvent` _returnvalue (delegate `OnPawnDetected`))
  ;; Sight Hearing and State Debug Draw
  (`|ExecutionSequence`
    (:`then_0`
      (if (`self.DrawDebugSight`)
        (`KismetSystemLibrary.DrawDebugConeInDegrees` (`KismetMathLibrary.MakeVector` _returnvalue_x _returnvalue_y (+ _returnvalue_z (`CapsuleComponent.CapsuleHalfHeight` (`Actor.GetComponentByClass` _owneractor "/Script/Engine.CapsuleComponent")))) (`Actor.GetActorForwardVector` _owneractor) (`self.SightRange`) _sightconeangle _sightconeangle 12 (struct :`G` 0.310141 :`B` 1.0 :`A` 1.0) 0.2)))
    (:`then_1`
      (if (`self.DrawMaxHearingRange`)
        (`KismetSystemLibrary.DrawDebugSphere` (`Actor.K2_GetActorLocation` (`self.OwnerActor`)) (`self.MaxHearingRange`) 12 (struct :`R` 0.946185 :`G` 1.0 :`A` 1.0) 0.2)))
    (:`then_2`
      (if (`self.DrawDebugState`)
        (bind _state (`self.GetCurrentState`))
        (`KismetSystemLibrary.DrawDebugString` (0.0 0.0 100.0) (`|GetEnumeratorNameAsString` _state) (`self.OwnerActor`) (struct :`R` 1.0 :`G` 1.0 :`B` 1.0 :`A` 1.0) DeltaSeconds)))))

(event `OnEnemyGradualDetected`
  ;[0 0.6252 0.849 0.5] Sight System
  ;; DetectionEvent
  (`self.OnEnemySeen` (`self.LastSeenActor`) :!label _label)
  (`self.HandleSensedSight` (`self.LastSeenActor`)))

(event `OnPawnDetected`
  (params (QueryInstance :type "EnvQueryInstanceBlueprintWrapper Object Reference") (QueryStatus :type "EEnvQueryStatus Enum" :default "Processing"))
  ;[0 0.6252 0.849 0.5] Sight System
  ;; Event when pawn is within Sight
  (bind _resultactors (`EnvQueryInstanceBlueprintWrapper.GetQueryResultsAsActors` QueryInstance))
  (for _array_element _resultactors
    ;; if detected pawn is of enemy faction, bind to the last seen actor
    (bind _isenemy (`self.FindIsFactionEnemy` _array_element))
    (if _isenemy
      (set `self.LastSeenActor` _array_element)
      (if (`self.InstantDetection`)
        (goto _label)
        (else
          ;;[0.4688 0.2397 0 0.5] Gradual Detection
          (`|ExecutionSequence`
            (:`then_0`
              (`/Engine/EditorBlueprintResources/StandardMacros.DoOnce` false :!label _label_2
                (:`Completed`
                  (message `/Game/EasyAiComponent/Blueprints/Helpers/BPI_EasyAI.StartDetection` (`Actor.GetComponentByClass` (`self.LastSeenActor`) "/Game/EasyAiComponent/Blueprints/OtherComponents/GradualDetection/BP_GradualDetectionComponent.BP_GradualDetectionComponent_C") (`self.OwnerPawn`)))))
            (:`then_1`
              (`KismetSystemLibrary.RetriggerableDelay` 0.5)
              (message `/Game/EasyAiComponent/Blueprints/Helpers/BPI_EasyAI.StopDetection` (`Actor.GetComponentByClass` (`self.LastSeenActor`) "/Game/EasyAiComponent/Blueprints/OtherComponents/GradualDetection/BP_GradualDetectionComponent.BP_GradualDetectionComponent_C"))
              (goto _label_2 :!via `Reset`))))))))

(event `OnRecieveNoiseEvent`
  (params (NoiseLocation :type "Vector Structure") (Instigator :type "Actor Object Reference") (OverrideNoiseAsEnemy :type Boolean))
  ;[0.08516 0.3854 0 0.5] Hearing System
  (if (< (`KismetMathLibrary.Vector_Distance` NoiseLocation (`Actor.K2_GetActorLocation` (`self.OwnerActor`))) (`self.MaxHearingRange`))
    ;; AI can hear if noise is made by enemy or if is overriding noise
    (bind _isenemy (`self.FindIsFactionEnemy` Instigator))
    (if (or _isenemy OverrideNoiseAsEnemy)
      ;; Noise heard event, sets noise location as point of interest
      (`self.OnNoiseHeard` NoiseLocation Instigator)
      (`self.HandleSensedNoise` NoiseLocation))))

(fn `AddCombatAction`
  (params (CombatAction :type "/Game/EasyAiComponent/CombatActions/S_CombatAction Structure (by ref)"))
  (returns (Index :type Integer))
  (bind _returnvalue (`KismetArrayLibrary.Array_Add` (`self.CombatActions`) CombatAction))
  (return _returnvalue))

(fn `ChangeBehavior`
  (params (BehaviorType :type "/Game/EasyAiComponent/Enums/E_BehaviorType Enum" :default "NewEnumerator0") (BehaviorTree :type "BehaviorTree Object Reference"))
  (bind _asbehavior_tree_component (cast `BehaviorTreeComponent` (`AIController.BrainComponent` (`self.OwnerAIController`))))
  (`BehaviorTreeComponent.SetDynamicSubtree` _asbehavior_tree_component (select `/Game/EasyAiComponent/Enums/E_BehaviorType` BehaviorType :`NewEnumerator0` (struct :`TagName` "Behavior.Idle") :`NewEnumerator1` (struct :`TagName` "Behavior.Patrol") :`NewEnumerator2` (struct :`TagName` "Behavior.Investigate") :`NewEnumerator3` (struct :`TagName` "Behavior.Combat") :!type "GameplayTag Structure") BehaviorTree))

(fn `ChangeCombatActions`
  (params (NewCombatActions :type "Array of /Game/EasyAiComponent/CombatActions/S_CombatAction Structure"))
  (returns (CombatActions :type "Array of /Game/EasyAiComponent/CombatActions/S_CombatAction Structure"))
  (bind _output_get (set `self.CombatActions` NewCombatActions))
  (return _output_get))

(fn `DoAttack`
  (params (CombatAction :type "/Game/EasyAiComponent/CombatActions/BP_BaseCombatAction Class Reference"))
  (bind _returnvalue (`|SpawnActorFromClass` CombatAction (`KismetMathLibrary.MakeTransform` (0.0 0.0 0.0)) "Undefined" "MultiplyWithRoot" null self null))
  (`/Game/EasyAiComponent/CombatActions/BP_BaseCombatAction.StartCombatAction` _returnvalue self)
  (`self.OnAttack`))

(fn `FindIsFactionEnemy`
  (params (TestedActor :type "Actor Object Reference"))
  (returns (IsEnemy :type Boolean))
  (locals (`L-IsEnemy` :type Boolean) (`L-TestedComponent` :type "/Game/EasyAiComponent/BP_EasyAiComponent Object Reference"))
  (bind _returnvalue (`Actor.GetComponentByClass` TestedActor "BP_EasyAiComponent_C"))
  (set `local.L-IsEnemy` false)
  (`/Engine/EditorBlueprintResources/StandardMacros.IsValid` _returnvalue
    (:`Is Valid`
      (set `local.L-TestedComponent` _returnvalue)
      (for _array_element (`/Game/EasyAiComponent/Data/Factions/PDA_Factions.EnemyFactions` (`self.Faction`))
        (if (== _array_element (`/Game/EasyAiComponent/BP_EasyAiComponent.Faction` (`local.L-TestedComponent`)))
          (set `local.L-IsEnemy` true)
          (break)))
      (return (`local.L-IsEnemy`)))
    (:`Is Not Valid`
      (if (and (`KismetArrayLibrary.Array_Contains` (`/Game/EasyAiComponent/Data/Factions/PDA_Factions.EnemyFactions` (`self.Faction`)) "/Game/EasyAiComponent/Data/Factions/DA_Faction_Player.DA_Faction_Player") (== (`local.TestedActor`) (`self.PlayerPawn`)))
        (set `local.L-IsEnemy` true)
        (return (`local.L-IsEnemy`))
        (else
          (return (`local.L-IsEnemy`)))))))

(fn `GetCurrentState`
  (returns (State :type "/Game/EasyAiComponent/Enums/E_AIStates Enum"))
  (return (cast `/Game/EasyAiComponent/Enums/E_AIStates` (`BlackboardComponent.GetValueAsEnum` (`self.OwnerBlackboard`) (`self.StateKeyName`)))))

(fn `GetPatrolRoute`
  (returns (PatrolRoute :type "/Game/EasyAiComponent/Blueprints/BP_PatrolRoute Object Reference"))
  (return (`self.PatrolRoute`)))

(fn `HandleActionStationFinished`
  (`self.OnFinishedUsingActionStation`)
  (`KismetSystemLibrary.PrintString` "ActionFinished"))

(fn `HandleSensedDamage`
  (params (DamagingActor :type "Actor Object Reference"))
  (bind (_outhit _returnvalue) (`KismetSystemLibrary.LineTraceSingle` :`Start` (`Actor.K2_GetActorLocation` (`self.OwnerActor`)) :`End` (`Actor.K2_GetActorLocation` DamagingActor) :`TraceChannel` "TraceTypeQuery1" :`DrawDebugType` "ForOneFrame"))
  (if _returnvalue
    (bind _state (`self.GetCurrentState`))
    (switch `/Game/EasyAiComponent/Enums/E_AIStates` _state
      (:`NewEnumerator0`
        (`self.SetStateAsInvestigative` (`.Location` (`GameplayStatics.BreakHitResult` _outhit)) :!label _label))
      (:`NewEnumerator1`
        (`self.SetStateAsAttacking` DamagingActor))
      (:`NewEnumerator3`
        (goto _label)))))

(fn `HandleSensedNoise`
  (params (Location :type "Vector Structure"))
  (bind _state (`self.GetCurrentState`))
  (switch `/Game/EasyAiComponent/Enums/E_AIStates` _state
    (:`NewEnumerator0`
      _)
    (:`NewEnumerator3`
      _))
  (`self.SetStateAsInvestigative` Location))

(fn `HandleSensedSight`
  (params (SeenActor :type "Actor Object Reference"))
  (bind _state (`self.GetCurrentState`))
  (switch `/Game/EasyAiComponent/Enums/E_AIStates` _state
    (:`NewEnumerator0`
      _)
    (:`NewEnumerator3`
      _))
  (`self.SetStateAsAttacking` SeenActor))

(fn `InitializeBehaviors`
  ; Behavior remains project default if Data is empty
  (`/Engine/EditorBlueprintResources/StandardMacros.IsValid` (`self.Behaviors`)
    (:`Is Valid`
      (`|ExecutionSequence`
        (:`then_0`
          ; Idle Behavior
          (`self.ChangeBehavior` "NewEnumerator0" (`/Game/EasyAiComponent/Data/Behaviors/PDA_Behaviors.IdleBehavior` (`self.Behaviors`))))
        (:`then_1`
          ; PatrolBehavior
          (`self.ChangeBehavior` "NewEnumerator1" (`/Game/EasyAiComponent/Data/Behaviors/PDA_Behaviors.PatrolBehavior` (`self.Behaviors`))))
        (:`then_2`
          ; Investigative Behavior
          (`self.ChangeBehavior` "NewEnumerator2" (`/Game/EasyAiComponent/Data/Behaviors/PDA_Behaviors.InvestigatingBehavior` (`self.Behaviors`))))
        (:`then_3`
          ; Combat Behavior
          (`self.ChangeBehavior` "NewEnumerator3" (`/Game/EasyAiComponent/Data/Behaviors/PDA_Behaviors.CombatBehavior` (`self.Behaviors`))))))))

(fn `InitializeBlackboardValues`
  ; Set Default attack range
  (`BlackboardComponent.SetValueAsFloat` (`self.OwnerBlackboard`) (`self.AttackRadiusKeyName`) (`self.BaseAttackRange`))
  ; Set range to retreat
  (`BlackboardComponent.SetValueAsFloat` (`self.OwnerBlackboard`) (`self.DefendRadiusKeyName`) (`self.RetreatDistance`)))

(fn `InitializeVariables`
  (bind _output_get (set `self.OwnerActor` (`self.GetOwner`)))
  ; Run EasyAi Main BT
  (bind _output_get_2 (set `self.OwnerAIController` (`AIBlueprintHelperLibrary.GetAIController` _output_get)))
  (`AIController.RunBehaviorTree` _output_get_2 "/Game/EasyAiComponent/BehaviorTrees/BT_EasyAI_Main.BT_EasyAI_Main")
  ; Establish References
  (set `self.OwnerBlackboard` (`AIController.Blackboard` (`self.OwnerAIController`)))
  (set `self.OwnerCharacterMovement` (`Actor.GetComponentByClass` (`self.OwnerActor`) "/Script/Engine.CharacterMovementComponent"))
  (set `self.PlayerPawn` (`GameplayStatics.GetPlayerPawn` 0))
  (bind _aspawn (cast `Pawn` (`self.OwnerActor`)))
  (set `self.OwnerPawn` _aspawn))

(fn `RemoveCombatActionByAction`
  (params (ActionToRemove :type "/Game/EasyAiComponent/CombatActions/S_CombatAction Structure (by ref)"))
  (`KismetArrayLibrary.Array_RemoveItem` (`self.CombatActions`) ActionToRemove))

(fn `RemoveCombatActionByIndex`
  (params (IndexToRemove :type Integer))
  (`KismetArrayLibrary.Array_Remove` (`self.CombatActions`) IndexToRemove))

(fn `ResetBehavior`
  (`self.SetStateAsPassive`)
  (`self.InitializeBehaviors`))

(fn `SetMovementSpeed`
  (params (Speed :type "/Game/EasyAiComponent/Enums/E_MovementSpeed Enum" :default "NewEnumerator0"))
  (returns (SpeedValue :type "Float (double-precision)"))
  (bind _output_get (set `CharacterMovementComponent.MaxWalkSpeed` (select `/Game/EasyAiComponent/Enums/E_MovementSpeed` Speed :`NewEnumerator1` (`self.WalkingSpeed`) :`NewEnumerator2` (`self.JoggingSpeed`) :`NewEnumerator3` (`self.SprintingSpeed`) :!type "Float (single-precision)") (`self.OwnerCharacterMovement`)))
  (return _output_get))

(fn `SetStateAsAttacking`
  (params (AttackTarget :type "Actor Object Reference"))
  (set `self.AttackTarget` AttackTarget)
  (`BlackboardComponent.SetValueAsEnum` (`self.OwnerBlackboard`) (`self.StateKeyName`) (enumliteral `/Game/EasyAiComponent/Enums/E_AIStates` "NewEnumerator1"))
  (`BlackboardComponent.SetValueAsObject` (`self.OwnerBlackboard`) (`self.AttackTargetKeyName`) (`self.AttackTarget`)))

(fn `SetStateAsDead`
  (`BlackboardComponent.SetValueAsEnum` (`self.OwnerBlackboard`) (`self.StateKeyName`) (enumliteral `/Game/EasyAiComponent/Enums/E_AIStates` "NewEnumerator4")))

(fn `SetStateAsInvestigative`
  (params (Location :type "Vector Structure"))
  (`BlackboardComponent.SetValueAsEnum` (`self.OwnerBlackboard`) (`self.StateKeyName`) (enumliteral `/Game/EasyAiComponent/Enums/E_AIStates` "NewEnumerator3"))
  (`BlackboardComponent.SetValueAsVector` (`self.OwnerBlackboard`) (`self.PointOfInterestKeyName`) Location))

(fn `SetStateAsPassive`
  (`BlackboardComponent.SetValueAsEnum` (`self.OwnerBlackboard`) (`self.StateKeyName`) (enumliteral `/Game/EasyAiComponent/Enums/E_AIStates` "NewEnumerator0")))