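; Manager actor that spawns customers at BP_CustomerSpawn and opens their dialogue.
; Once started, a looping timer calls CreateCustomer, which uses supplied customer data or randomizes identity, appearance and interaction with a base rent dialogue, then tracks each customer.
; StartDialogue fills the HUD with the first line, runs the dialogue's start-action actor, plays voice and switches to UI input.
; Tick prints spawn timer state for debugging.
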(event `self.ReceiveBeginPlay`
  ; Swap with player BP
  (bind _asbp_first_person_character (cast `/Game/FirstPerson/Blueprints/BP_FirstPersonCharacter` (`GameplayStatics.GetPlayerCharacter` 0)))
  (set `self.PlayerRef` _asbp_first_person_character))

(event `StartCustomerSpawn`
  (`KismetSystemLibrary.K2_SetTimerDelegate` (delegate `CustomerSpawn`) 0.5 true))

(event `self.ReceiveTick`
  (params (DeltaSeconds :type "Float (single-precision)"))
  (bind _spawntimer (`self.SpawnTimer`))
  (`KismetSystemLibrary.PrintString` (`KismetStringLibrary.Conv_BoolToString` (`KismetSystemLibrary.K2_IsValidTimerHandle` _spawntimer)))
  (`KismetSystemLibrary.PrintString` (`KismetStringLibrary.Conv_DoubleToString` (`KismetSystemLibrary.K2_GetTimerElapsedTimeHandle` _spawntimer))))

(event `CustomerSpawn`
  (`self.CreateCustomer` null))

(fn `CreateCustomer`
  (params (CustomerData :type "/Game/Data/Customers/PDA_Customer Object Reference"))
  (bind (_mesh _icon) (`self.RandomCustomerAppearance`))
  (`/Engine/EditorBlueprintResources/StandardMacros.IsValid` CustomerData
    (:`Is Valid`
      (bind _returnvalue (`|SpawnActorFromClass` "/Game/Blueprints/Character/BP_Customer.BP_Customer_C" (`self.GetCustomerSpawnTransform`) "AlwaysSpawn" "MultiplyWithRoot" null (`/Game/Data/Customers/PDA_Customer.CustomerInfo` CustomerData) null))
      (`KismetArrayLibrary.Array_Add` (`self.Customers`) _returnvalue))
    (:`Is Not Valid`
      (bind _returnvalue_2 (`|SpawnActorFromClass` "/Game/Blueprints/Character/BP_Customer.BP_Customer_C" (`self.GetCustomerSpawnTransform`) "AdjustIfPossibleButAlwaysSpawn" "MultiplyWithRoot" null (make `/Game/Blueprints/Struct/S_CustomerInfo` (`self.RandomCustomerName`) (`self.RandomCustomerID`) (`self.RandomCustomerPhone`) _mesh _icon "/Game/Data/Dialogue/DA_Rent_Base.DA_Rent_Base" (`self.RandomIneraction`)) null))
      (`KismetArrayLibrary.Array_Add` (`self.Customers`) _returnvalue_2))))

(fn `GetCustomerSpawnTransform`
  (returns (ReturnValue :type "Transform Structure (by ref)"))
  (bind _returnvalue (`GameplayStatics.GetActorOfClass` "/Game/Blueprints/BP_CustomerSpawn.BP_CustomerSpawn_C"))
  (return (`self.GetTransform` _returnvalue)))

(fn `RandomCustomerAppearance`
  (returns (Mesh :type "SkeletalMesh Object Reference") (Icon :type "Texture2D Object Reference"))
  (locals (RandomMesh :type "SkeletalMesh Object Reference"))
  (bind _randomappearance (`self.RandomAppearance`))
  (bind _keys (`BlueprintMapLibrary.Map_Keys` _randomappearance))
  (bind _output_get (set `local.RandomMesh` (`KismetArrayLibrary.Array_Random` _keys)))
  (return _output_get (`BlueprintMapLibrary.Map_Find` _randomappearance _output_get)))

(fn `RandomCustomerID`
  (returns (Result :type Text))
  (return (`|FormatText` "{1}{2}{3}{4}{5}" (`KismetMathLibrary.RandomIntegerInRange` 0 9) (`KismetMathLibrary.RandomIntegerInRange` 0 9) (`KismetMathLibrary.RandomIntegerInRange` 0 9) (`KismetMathLibrary.RandomIntegerInRange` 0 9) (`KismetMathLibrary.RandomIntegerInRange` 0 9))))

(fn `RandomCustomerName`
  (returns (Result :type Text))
  (return (`|FormatText` "{FirstName} {LastName}" (`KismetArrayLibrary.Array_Random` (`self.RandomFirstName`)) (`KismetArrayLibrary.Array_Random` (`self.RandomSecondName`)))))

(fn `RandomCustomerPhone`
  (returns (Result :type Text))
  (return (`|FormatText` "{1}-{2}-{3}{4}{5}{6}" (select `int` (`KismetMathLibrary.RandomIntegerInRange` 0 4) :`0` 303 :`1` 719 :`2` 720 :`3` 970 :`4` 983) (`KismetMathLibrary.RandomIntegerInRange` 100 999) (`KismetMathLibrary.RandomIntegerInRange` 0 9) (`KismetMathLibrary.RandomIntegerInRange` 0 9) (`KismetMathLibrary.RandomIntegerInRange` 0 9) (`KismetMathLibrary.RandomIntegerInRange` 0 9))))

(fn `RandomIneraction`
  (returns (ReturnValue :type "/Game/Blueprints/Enums/E_CustomerInteraction Enum"))
  (return (cast `/Game/Blueprints/Enums/E_CustomerInteraction` (`KismetMathLibrary.Conv_IntToByte` (`KismetMathLibrary.RandomIntegerInRange` 0 5)))))

(fn `StartDialogue`
  (params (CustomerInfo :type "/Game/Blueprints/Struct/S_CustomerInfo Structure"))
  (bind _returnvalue (`GameplayStatics.GetPlayerController` 0))
  (bind _dialoguewidget (`self.DialogueWidget`))
  (bind (_name _customerid _phonenumber _mesh _icon _dialogue) (break `/Game/Blueprints/Struct/S_CustomerInfo` (`local.CustomerInfo`)))
  (bind (_dialogueline _voiceline) (break `/Game/Systems/Dialogue/Blueprints/Struct/S_DialogueLine` (`|GetArrayItem` (`/Game/Data/Dialogue/PDA_Dialogue.Lines` (`.Dialogue_14_25D717834DE63754B9437D938897FD67` (break `/Game/Blueprints/Struct/S_CustomerInfo` (`local.CustomerInfo`)))))))
  (`/Engine/EditorBlueprintResources/StandardMacros.IsValid` (`self.DialogueWidget`)
    (:`Is Valid`
      _)
    (:`Is Not Valid`
      (bind _returnvalue_2 (`|CreateWidget` "/Game/Systems/Dialogue/UI/WBP_DialogueHUD.WBP_DialogueHUD_C" (`GameplayStatics.GetPlayerController` 0)))
      (set `self.DialogueWidget` _returnvalue_2)))
  (`TextBlock.SetText` (`/Game/Systems/Dialogue/UI/WBP_DialogueHUD.SpeakerName` _dialoguewidget) _name)
  (`TextBlock.SetText` (`/Game/Systems/Dialogue/UI/WBP_DialogueHUD.LineText` _dialoguewidget) _dialogueline)
  (`|ExecutionSequence`
    (:`then_0`
      (bind _returnvalue_3 (`|SpawnActorFromClass` (`/Game/Data/Dialogue/PDA_Dialogue.OnDialogueStartedAction` _dialogue) (`KismetMathLibrary.MakeTransform` (0.0 0.0 0.0)) "AlwaysSpawn" "MultiplyWithRoot" null null))
      (`/Game/Systems/Dialogue/Blueprints/Actions/BP_DialogueAction_Base.ExecuteDialogueAction` _returnvalue_3))
    (:`then_1`
      (`UserWidget.AddToViewport` (`self.DialogueWidget`) 0)
      (`GameplayStatics.PlaySound2D` _voiceline 1.0 1.0 0.0 null null)
      (`WidgetBlueprintLibrary.SetInputMode_UIOnlyEx` _returnvalue (`self.DialogueWidget`) "DoNotLock" true)
      (set `PlayerController.bShowMouseCursor` true _returnvalue))))

(fn `UserConstructionScript`)