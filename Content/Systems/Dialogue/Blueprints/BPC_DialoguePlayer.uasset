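; BPC_DialoguePlayer is a component for BP_FirstPersonCharacter that handles the player's interact input.
; On BeginPlay it caches the owning character and adds the dialogue input mapping context.
; IA_Interact sphere-traces from the camera on the Visibility channel, with debug drawing, and sends the hit actor an OnInteract message carrying the player.
; A debug key tells BP_CustomerManager to start spawning customers.
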(event `self.ReceiveBeginPlay`
  (bind _asbp_first_person_character (cast `/Game/FirstPerson/Blueprints/BP_FirstPersonCharacter` (`self.GetOwner`)))
  (set `self.PlayerBP` _asbp_first_person_character)
  (`EnhancedInputSubsystemInterface.AddMappingContext` (pcsubsystem `EnhancedInputLocalPlayerSubsystem` (`GameplayStatics.GetPlayerController` 0)) "/Game/Systems/Dialogue/Inputs/IMC_Dialogue.IMC_Dialogue" 0 (struct)))

(event `EnhancedInput|/Game/Systems/Dialogue/Inputs/InputActions/IA_Interact`
  (params (ActionValue :type Boolean) (ElapsedSeconds :type "Float (double-precision)") (TriggeredSeconds :type "Float (double-precision)") (InputAction :type "InputAction Object Reference" :default "/Game/Systems/Dialogue/Inputs/InputActions/IA_Interact.IA_Interact"))
  (bind _returnvalue (`GameplayStatics.GetPlayerCameraManager` 0))
  (bind _returnvalue_2 (`PlayerCameraManager.GetCameraLocation` _returnvalue))
  (:`Started`
    (bind (_outhit _returnvalue_3) (`KismetSystemLibrary.SphereTraceSingle` :`Start` _returnvalue_2 :`End` (+ _returnvalue_2 (* (`Actor.GetActorForwardVector` _returnvalue) (`self.InteractDistance`))) :`Radius` 30.0 :`TraceChannel` "TraceTypeQuery1" :`DrawDebugType` "ForDuration"))
    (if _returnvalue_3
      (message `/Game/Blueprints/Helpers/BPI_Interaction.OnInteract` (`.HitActor` (`GameplayStatics.BreakHitResult` _outhit)) (`self.PlayerBP`)))))

(event `EnhancedInput|/Game/Systems/Dialogue/Inputs/InputActions/IA_DebugKey1`
  (params (ActionValue :type Boolean) (ElapsedSeconds :type "Float (double-precision)") (TriggeredSeconds :type "Float (double-precision)") (InputAction :type "InputAction Object Reference" :default "/Game/Systems/Dialogue/Inputs/InputActions/IA_DebugKey1.IA_DebugKey1"))
  (:`Started`
    (bind _returnvalue (`GameplayStatics.GetActorOfClass` "/Game/Systems/Dialogue/Blueprints/Managers/BP_CustomerManager.BP_CustomerManager_C"))
    (`/Game/Systems/Dialogue/Blueprints/Managers/BP_CustomerManager.StartCustomerSpawn` _returnvalue)))