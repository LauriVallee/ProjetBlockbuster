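; BP_Customer is a customer character that carries a CustomerData record and opens dialogue when interacted with.
; On BeginPlay it finds the BP_CustomerManager in the level and prints its name, ID, phone number and main interaction to screen.
; OnInteract passes its CustomerData to the manager's StartDialogue, leaving the conversation logic to the manager.
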(event `self.ReceiveBeginPlay`
  (bind (_name _customerid _phonenumber _mesh _icon _dialogue _maininteraction) (break `/Game/Blueprints/Struct/S_CustomerInfo` (`self.CustomerData`)))
  (bind _returnvalue (`GameplayStatics.GetActorOfClass` "/Game/Systems/Dialogue/Blueprints/Managers/BP_CustomerManager.BP_CustomerManager_C"))
  (set `self.CustomerManagerRef` _returnvalue)
  (`KismetSystemLibrary.PrintString` (`KismetTextLibrary.Conv_TextToString` _name))
  (`KismetSystemLibrary.PrintString` (`KismetTextLibrary.Conv_TextToString` _customerid))
  (`KismetSystemLibrary.PrintString` (`KismetTextLibrary.Conv_TextToString` _phonenumber))
  (`KismetSystemLibrary.PrintString` (`|GetEnumeratorNameAsString` _maininteraction)))

(event `/Game/Blueprints/Helpers/BPI_Interaction.OnInteract`
  (params (Instigator :type "Actor Object Reference"))
  (`/Game/Systems/Dialogue/Blueprints/Managers/BP_CustomerManager.StartDialogue` (`self.CustomerManagerRef`) (`self.CustomerData`)))

(fn `UserConstructionScript`)